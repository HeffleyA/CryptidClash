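; King of the Hill game state for Cryptid Clash that scores players each second.
; A looping timer walks the PlayerArray and adds a point to each BP_KOTH_PlayerState found in the first BP_Hill's overlapping players.
; Players off the hill drop straight to zero, because the decrement is clamped between 0 and 0.
; The check for reaching 100 points leads to no action.
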(event `self.ReceiveBeginPlay`
  (`KismetSystemLibrary.K2_SetTimerDelegate` (delegate `UpdateKOTHScoring`) 1.0 true))

(event `UpdateKOTHScoring`
  (bind _outactors (`GameplayStatics.GetAllActorsOfClass` "/Game/CryptidClash/Blueprints/BP_Hill.BP_Hill_C"))
  (for _array_element (`self.PlayerArray`)
    (bind _asbp_koth_player_state (cast `/Game/CryptidClash/Blueprints/BP_KOTH_PlayerState` _array_element))
    (if (`KismetArrayLibrary.Array_Contains` (`/Game/CryptidClash/Blueprints/BP_Hill.OverlappingPlayers` (`|GetArrayItem` _outactors)) _asbp_koth_player_state)
      (bind _currentpoints (`/Game/CryptidClash/Blueprints/BP_KOTH_PlayerState.CurrentPoints` _asbp_koth_player_state))
      (set `/Game/CryptidClash/Blueprints/BP_KOTH_PlayerState.CurrentPoints` (+ _currentpoints 1) _asbp_koth_player_state)
      (if (== _currentpoints 100)
        _)
      (else
        (set `/Game/CryptidClash/Blueprints/BP_KOTH_PlayerState.CurrentPoints` (`KismetMathLibrary.Clamp` (- _currentpoints 1)) _asbp_koth_player_state)))))

(event `self.ReceiveTick`
  (params (DeltaSeconds :type "Float (single-precision)")))

(fn `UserConstructionScript`)