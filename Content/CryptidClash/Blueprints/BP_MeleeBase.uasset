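; Base melee weapon Blueprint that supplies a hit-detection trace for weapons in CryptidClash.
; TraceForTargets sphere-traces for Pawns between the mesh's S_Base and S_Tip sockets.
; As wired, hits that are already in HitActors and implement BPI_Damageable are re-added to that array and trigger ApplyDamage, which has no inputs set.
; Nothing in this Blueprint calls the trace, and its events are empty.
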(fn `TraceForTargets`
  (bind _hitactors (`self.HitActors`))
  (bind _outhits (`KismetSystemLibrary.SphereTraceMultiForObjects` (`SceneComponent.GetSocketLocation` (`self.StaticMesh`) "S_Base") (`SceneComponent.GetSocketLocation` (`self.StaticMesh`) "S_Tip") 0.0 (`|MakeArray` "ObjectTypeQuery3" :!type "EObjectTypeQuery Enum")))
  (for _array_element _outhits
    (bind (_bblockinghit _binitialoverlap _time _distance _location _impactpoint _normal _impactnormal _physmat _hitactor) (`GameplayStatics.BreakHitResult` _array_element))
    (if (and (!= (`KismetArrayLibrary.Array_Contains` _hitactors _hitactor) false) (`KismetSystemLibrary.DoesImplementInterface` _hitactor "/Game/CryptidClash/Blueprints/BPI_Damageable.BPI_Damageable_C"))
      (`KismetArrayLibrary.Array_Add` _hitactors _hitactor)
      (`GameplayStatics.ApplyDamage` null))))

(fn `UserConstructionScript`)