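; BP_Hill is the King of the Hill zone actor that tracks which players are standing inside it.
; Begin and end overlap events cast the other actor to a Pawn, then its PlayerState to BP_KOTH_PlayerState, and add it to or remove it from OverlappingPlayers.
; The Blueprint only maintains this list and contains no scoring logic, with BeginPlay, Tick and the construction script left empty.
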(event `self.ReceiveActorBeginOverlap`
  (params (OtherActor :type "Actor Object Reference"))
  (bind _aspawn (cast `Pawn` OtherActor))
  (bind _asbp_koth_player_state (cast `/Game/CryptidClash/Blueprints/BP_KOTH_PlayerState` (`Pawn.PlayerState` _aspawn)))
  (`KismetArrayLibrary.Array_Add` (`self.OverlappingPlayers`) _asbp_koth_player_state))

(event `self.ReceiveActorEndOverlap`
  (params (OtherActor :type "Actor Object Reference"))
  (bind _aspawn (cast `Pawn` OtherActor))
  (bind _asbp_koth_player_state (cast `/Game/CryptidClash/Blueprints/BP_KOTH_PlayerState` (`Pawn.PlayerState` _aspawn)))
  (`KismetArrayLibrary.Array_RemoveItem` (`self.OverlappingPlayers`) _asbp_koth_player_state))

(fn `UserConstructionScript`)